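; AI task action that sends a Peon agent to the door of a Base.
; On start it gets the first Base through the Peon and stores that door's position with Z flattened to zero.
; Each Execute call prints a French debug message and issues AIMoveTo toward the stored point, setting the step to Finished when the move succeeds.
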(event EventExecute
  (params (owner :type Pawn%20Object%20Reference) (DeltaTime :type Float%20%28single-precision%29))
  (Development|PrintString 0 "Je vais a la base :)" true true "(R=0.000000,G=0.660000,B=1.000000,A=1.000000)" DeltaTime)
  (AI|AIMoveTo owner owner (Variables|Default|GetDoorPos) 0 5.0 false
    (:OnSuccess
      (Variables|Default|SetcurrentStep "Finished"))))

(event EventStartTask
  (params (owner :type Pawn%20Object%20Reference))
  (bind _asaiagent (Utilities|Casting|CastToAIAgent owner))
  (bind _aspeon (Utilities|Casting|CastToPeon _asaiagent))
  (bind _actor (Default|GetFirstActor _aspeon "/Game/Blueprints/Base.Base_C"))
  (bind _asbase (Utilities|Casting|CastToBase _actor))
  (bind _doorpos (Default|GetDoorPos _asbase))
  (Variables|Default|SetDoorPos (Math|Vector|MakeVector (.X (Class|KismetMathLibrary|BreakVector3f _doorpos)) (.Y (Class|KismetMathLibrary|BreakVector3f _doorpos)) 0.0)))