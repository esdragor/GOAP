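; BP_CutTree is a timed action that stands in for chopping down a tree.
; StartTask resets a countdown from MaxTimer, and Execute decrements it by DeltaTime each tick while printing a "chop chop" debug message.
; When the countdown drops below zero, it sets CurrentStep to Finished to end the action.
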(event EventExecute
  (params (owner :type Pawn%20Object%20Reference) (DeltaTime :type Float%20%28single-precision%29))
  (Variables|Default|SettimerRemaining (- (Variables|Default|GettimerRemaining) DeltaTime))
  (Development|PrintString 0 "chop chop" true true "(R=0.000000,G=0.660000,B=1.000000,A=1.000000)" DeltaTime)
  (if (< (Variables|Default|GettimerRemaining) 0.0)
    (Variables|Default|SetcurrentStep "Finished")))

(event EventStartTask
  (params (owner :type Pawn%20Object%20Reference))
  (Variables|Default|SettimerRemaining (Variables|Default|GetmaxTimer)))