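; BP_GoToForest is an AI task that sends a Peon to a nearby forest.
; StartTask casts the owner to Peon, finds the RessourcesManager, and stores the result of its GetNearForest query for the owner's location.
; Execute prints a French debug message and calls AIMoveTo toward that forest, marking the step Finished on success, with no failure handling.
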(event EventExecute
  (params (owner :type Pawn%20Object%20Reference) (DeltaTime :type Float%20%28single-precision%29))
  (Development|PrintString 0 "Je vais dans la foret :)" true true "(R=0.000000,G=0.660000,B=1.000000,A=1.000000)" DeltaTime)
  (AI|AIMoveTo owner owner (Variables|Default|GetForest) 0 5.0 false
    (:OnSuccess
      (Variables|Default|SetcurrentStep "Finished"))))

(event EventStartTask
  (params (owner :type Pawn%20Object%20Reference))
  (bind _asaiagent (Utilities|Casting|CastToAIAgent owner))
  (bind _aspeon (Utilities|Casting|CastToPeon _asaiagent))
  (bind _actor (Default|GetFirstActor _aspeon "/Game/Blueprints/RessourcesManager.RessourcesManager_C"))
  (bind _asressources_manager (Utilities|Casting|CastToRessourcesManager _actor))
  (bind _nearpos (Default|GetNearForest _asressources_manager (Transformation|GetActorLocation owner)))
  (Variables|Default|SetForest _nearpos))