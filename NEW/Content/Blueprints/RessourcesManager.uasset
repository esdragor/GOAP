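; RessourcesManager is a Blueprint that locates forest resources in the world, exposing a lookup for the one closest to a pawn.
; GetNearForest loops over the Forest array, keeps the entry with the smallest distance below Dist to the given position, and returns that actor's location.
; The construction script is empty.
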(fn ConstructionScript)

(fn GetNearForest
  (params (PawnPos :type Vector))
  (for _array_element (Variables|Default|GetForest)
    (if (< (Math|Vector|Distance(Vector) PawnPos (Transformation|GetActorLocation _array_element)) (LocalVariables|GetDist))
      (LocalVariables|SetDist (Math|Vector|Distance(Vector) PawnPos (Transformation|GetActorLocation _array_element)))
      (LocalVariables|SetSelectedSpawn _array_element)))
  (return (Transformation|GetActorLocation (LocalVariables|GetSelectedSpawn))))